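; MySProjectile is a timed explosive actor that detonates half a second after spawning, despite its projectile name.
; On BeginPlay it waits, spawns an explosion emitter, applies radial damage from the Damg and Radius variables, and fires a radial force impulse.
; It then draws a debug sphere at the blast point and destroys itself.
; Damg and Radius have RepNotify functions, both empty.
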(event EventBeginPlay
  (bind _returnvalue (Transformation|GetActorLocation))
  (Utilities|FlowControl|Delay 0.5)
  (Effects|SpawnEmitteratLocation "/Game/WeaponEffects/Explosion/P_Explosion.P_Explosion" _returnvalue)
  (Game|Damage|ApplyRadialDamage (Variables|Default|GetDamg) _returnvalue (Variables|Default|GetRadius) 0 0 self (Game|GetInstigatorController) false "ECC_Visibility")
  (Class|RadialForceComponent|FireImpulse (Variables|Default|GetRadialForce))
  (Rendering|Debug|DrawDebugSphere _returnvalue 1e+02 12 "(R=0.995748,G=1.000000,B=0.000000,A=1.000000)" 1.0)
  (Actor|DestroyActor))

(fn ConstructionScript)

(fn OnRepDamg)

(fn OnRepRadius)