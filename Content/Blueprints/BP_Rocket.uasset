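; BP_Rocket is an actor that explodes on a fixed short timer after it begins play.
; BeginPlay waits one second, then calls the Explode event.
; Explode spawns an explosion particle, applies radial damage credited to the instigator's controller, draws a debug sphere of the damage radius, and destroys the actor.
; The file contains no movement or impact logic.
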(event Custom|Explode
  (bind _returnvalue (Transformation|GetActorLocation))
  (bind _damage_radius (Variables|Default|GetDamage%20Radius))
  (Effects|SpawnEmitteratLocation "/Game/WeaponEffects/Explosion/P_Explosion.P_Explosion" _returnvalue)
  (Game|Damage|ApplyRadialDamage 1e+02 _returnvalue _damage_radius 0 0 self (Game|GetInstigatorController) false "ECC_Visibility")
  (Rendering|Debug|DrawDebugSphere _returnvalue _damage_radius 12 "(R=0.995748,G=1.000000,B=0.000000,A=1.000000)" 1.0)
  (Actor|DestroyActor))

(event EventBeginPlay
  (Utilities|FlowControl|Delay 1.0)
  (CallFunction|Explode))

(fn ConstructionScript)